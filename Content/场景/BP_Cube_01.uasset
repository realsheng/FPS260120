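; BP_Cube_01 is a network replication test actor that shows its authority and a replicated value through text renders.
; On BeginPlay it checks the local role, labels TextRender as Authority or No Authority, and prints server or client.
; TextRender1 displays RepValue, written at BeginPlay by 更新RepValue and again by the OnRep_RepValue notify.
; Nothing in this graph changes RepValue, and Tick is empty.
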(event `self.ReceiveBeginPlay`
  (bind _textrender (`self.TextRender`))
  (`self.更新RepValue`)
  (if (`|EnumEquality` (`self.GetLocalRole`) "ROLE_Authority")
    (`TextRenderComponent.K2_SetText` _textrender "Authority")
    (`KismetSystemLibrary.PrintString` "server" true true (struct :`G` 0.66 :`B` 1.0 :`A` 1.0) 10.0)
    (else
      (`TextRenderComponent.K2_SetText` _textrender "No Authority")
      (`KismetSystemLibrary.PrintString` "client" true true (struct :`G` 0.66 :`B` 1.0 :`A` 1.0) 10.0))))

(event `更新RepValue`
  (`TextRenderComponent.K2_SetText` (`self.TextRender1`) (`KismetTextLibrary.Conv_StringToText` (`KismetStringLibrary.Concat_StrStr` "Rplicated:" (`KismetStringLibrary.Conv_IntToString` (`self.RepValue`))))))

(event `self.ReceiveTick`
  (params (DeltaSeconds :type "Float (single-precision)")))

(fn `OnRep_RepValue`
  (`TextRenderComponent.K2_SetText` (`self.TextRender1`) (`KismetTextLibrary.Conv_StringToText` (`KismetStringLibrary.Concat_StrStr` "Rplicated:" (`KismetStringLibrary.Conv_IntToString` (`self.RepValue`))))))

(fn `UserConstructionScript`)