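; Bullet actor (子弹_BP) that applies damage and impact feedback on hit.
; On the server, a tiny sphere trace at the hit point finds the target, damaging 玩家_BP or 敌人_BP depending on the game instance's 是否联网 (networked) check.
; Lethal hits credit a kill to the instigator's player state.
; Surface type picks the impact particle, multicast along with bullet-hole decals on hard surfaces, before the bullet destroys itself.
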(event `self.ReceiveHit`
  (params (MyComp :type "PrimitiveComponent Object Reference") (Other :type "Actor Object Reference") (OtherComp :type "PrimitiveComponent Object Reference") (bSelfMoved :type Boolean) (HitLocation :type "Vector Structure") (HitNormal :type "Vector Structure") (NormalImpulse :type "Vector Structure") (Hit :type "HitResult Structure (by ref)"))
  (bind `_攻击力` (`self.攻击力`))
  (bind `_攻击力_2` (`self.攻击力`))
  (`/Engine/EditorBlueprintResources/ActorMacros.Switch Has Authority`
    (:`Authority`
      (bind (_outhit _returnvalue) (`KismetSystemLibrary.SphereTraceSingle` HitLocation HitLocation 3.0 "TraceTypeQuery5"))
      (if _returnvalue
        (bind `_asfps_游戏实例` (cast `/Game/关卡/FPS_游戏实例` (`GameplayStatics.GetGameInstance`)))
        (`/Game/关卡/FPS_游戏实例.是否联网` `_asfps_游戏实例`
          (:`then`
            (bind (_bblockinghit _binitialoverlap _time _distance _location _impactpoint _normal _impactnormal _physmat _hitactor) (`GameplayStatics.BreakHitResult` _outhit))
            (bind `_as玩家_bp` (cast `/Game/玩家蓝图/玩家_BP` _hitactor)
              (:`then`
                (bind `_生命值` (`/Game/玩家蓝图/玩家_BP.生命值` `_as玩家_bp`))
                (if (<= `_生命值` `_攻击力_2`)
                  (if (not (== `_生命值` 0))
                    (bind `_as玩家_bp_2` (cast `/Game/玩家蓝图/玩家_BP` (`self.GetInstigator`)))
                    (bind `_asfps_玩家状态` (cast `/Game/关卡/FPS_玩家状态` (`Pawn.PlayerState` `_as玩家_bp_2`)))
                    (`/Game/关卡/FPS_玩家状态.杀敌数加一_OnServer` `_asfps_玩家状态`)
                    (`/Game/玩家蓝图/玩家_BP.生命值降低` `_as玩家_bp` (`KismetMathLibrary.FTrunc` `_攻击力_2`) :!label _label))
                  (else
                    (goto _label))))
              (:`CastFailed`
                _)))
          (:`else`
            (bind `_as敌人_bp` (cast `/Game/敌人蓝图/敌人_BP` _hitactor)
              (:`then`
                (bind `_生命值_2` (`/Game/敌人蓝图/敌人_BP.生命值` `_as敌人_bp`))
                (if (<= `_生命值_2` `_攻击力`)
                  (if (not (== `_生命值_2` 0))
                    (bind `_as玩家_bp_3` (cast `/Game/玩家蓝图/玩家_BP` (`self.GetInstigator`)))
                    (bind `_asfps_玩家状态_2` (cast `/Game/关卡/FPS_玩家状态` (`Pawn.PlayerState` `_as玩家_bp_3`)))
                    (`/Game/关卡/FPS_玩家状态.杀敌数加一_OnServer` `_asfps_玩家状态_2`)
                    (`/Game/敌人蓝图/敌人_BP.生命值降低` `_as敌人_bp` (`KismetMathLibrary.FTrunc` `_攻击力`) :!label _label_2))
                  (else
                    (goto _label_2))))
              (:`CastFailed`
                _))))
        (switch `EPhysicalSurface` (`GameplayStatics.GetSurfaceType` _outhit)
          (:`SurfaceType_Default`
            (set `self.命中特效` "/Game/Weapon_Impacts/Systems/Metal/Metal_Impact_Directional_01.Metal_Impact_Directional_01")
            (bind _returnvalue_2 (`KismetMathLibrary.Conv_VectorToRotator` _normal))
            (`self.生成弹孔贴花_Multicast` _location _returnvalue_2 :!label _label_3))
          (:`SurfaceType1`
            (set `self.命中特效` "/Game/Weapon_Impacts/Systems/Metal/Metal_Impact_Directional_03.Metal_Impact_Directional_03")
            (goto _label_3))
          (:`SurfaceType2`
            (set `self.命中特效` "/Game/Weapon_Impacts/Systems/Concrete/Concrete_Impact_Directional_01.Concrete_Impact_Directional_01")
            (goto _label_3))
          (:`SurfaceType3`
            (set `self.命中特效` "/Game/Weapon_Impacts/Systems/Water/Water_Impact_Base_01.Water_Impact_Base_01"))
          (:`SurfaceType4`
            (set `self.命中特效` "/Game/Weapon_Impacts/Systems/Dirt/Dirt_Impact_Directional_01.Dirt_Impact_Directional_01"))
          (:`SurfaceType5`
            (set `self.命中特效` "/Game/Weapon_Impacts/Systems/Wood/Impact_Wood_Directional_01.Impact_Wood_Directional_01")
            (goto _label_3))
          (:`SurfaceType6`
            (set `self.命中特效` "/Game/Weapon_Impacts/Systems/Grass/Grass_Impact_Directional_01.Grass_Impact_Directional_01"))
          (:`SurfaceType7`
            (set `self.命中特效` "/Game/Weapon_Impacts/Systems/Blood/Blood_Impact_Directional_01.Blood_Impact_Directional_01")))
        (`self.播放命中特效_Multicast` _location _returnvalue_2)
        (`self.K2_DestroyActor`)))))

(event `生成弹孔贴花_Multicast`
  (params (Location :type "Vector Structure") (Rotation :type "Rotator Structure"))
  ;[1 1 1] 生成弹孔贴花_Multicast
  (`GameplayStatics.SpawnDecalAtLocation` (`self.弹孔贴花`) (7.0 7.0 7.0) Location Rotation 5.0))

(event `播放命中特效_Multicast`
  (params (Location :type "Vector Structure") (Rotation :type "Rotator Structure"))
  ;[1 1 1] 播放命中特效_Multicast
  (`GameplayStatics.SpawnEmitterAtLocation` (`self.命中特效`) Location Rotation))

(fn `UserConstructionScript`)