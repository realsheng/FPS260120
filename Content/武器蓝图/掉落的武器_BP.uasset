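; Dropped weapon pickup actor that represents a weapon lying in the world, configured by a weapon data asset.
; On authority, its Construction Script sets the static mesh from that asset, printing an error if the mesh is invalid.
; Highlight events set or clear an interaction overlay material on the mesh.
; Getters expose magazine ammo, picked-up state and the data asset, and macros provide authority and autonomous-proxy role checks.
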(event `/Game/接口/掉落的武器接口.高亮显示`
  (`MeshComponent.SetOverlayMaterial` (`self.StaticMesh`) "/Game/材质/交互材质.交互材质"))

(event `/Game/接口/掉落的武器接口.关闭高亮`
  (`MeshComponent.SetOverlayMaterial` (`self.StaticMesh`) null))

(fn `UserConstructionScript`
  (`self.服务器端权威检测`
    (:`真`
      (bind `_静态` (`/Game/数据资产/武器_数据资产.静态` (`self.武器数据资产`))
        (:`then`
          (`StaticMeshComponent.SetStaticMesh` (`self.StaticMesh`) `_静态`))
        (:`else`
          (`KismetSystemLibrary.PrintString` "静态无效"))))))

(fn `获取弹匣子弹数量`
  (returns (`弹匣子弹数量` :type Integer))
  (return (`self.弹匣子弹数量`)))

(fn `获取是否被拾取过`
  (returns (`是否被拾取过` :type Boolean))
  (return (`self.是否被拾取过`)))

(fn `获取武器数据资产`
  (returns (`武器数据资产` :type "/Game/数据资产/武器_数据资产 Object Reference"))
  (return (`self.武器数据资产`)))