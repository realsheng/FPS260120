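; Equipped weapon actor that handles firing, magazine ammo and reload animation, with the server filling the magazine from a weapon data asset.
; Firing traces from the camera, then spawns a damage-carrying bullet from the muzzle toward that aim point and ejects a randomly pitched shell.
; An empty magazine plays a dry-fire sound and returns false.
; Effects play directly and through multicasts, most limited to remote machines.
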(event `self.ReceiveBeginPlay`
  ;[1 1 1] 获取武器数据资产
  (`/Engine/EditorBlueprintResources/ActorMacros.Switch Has Authority`
    (:`Authority`
      (set `self.弹匣子弹数量` (`/Game/数据资产/武器_数据资产.弹匣上限` (`self.武器数据资产`))))))

(event `/Game/接口/装备的的武器接口.武器换弹`
  ;[1 1 1] 武器换弹
  (`self.武器换弹_Multicast`)
  (`SkeletalMeshComponent.PlayAnimation` (`self.SkeletalMesh`) (`self.武器换弹动画`) false))

(event `武器换弹_Multicast`
  ;[1 1 1] 武器换弹_Multicast
  (`/Engine/EditorBlueprintResources/ActorMacros.Switch Has Authority`
    (:`Remote`
      (`SkeletalMeshComponent.PlayAnimation` (`self.SkeletalMesh`) (`self.武器换弹动画`) false))))

(event `播放开火特效_Multicast`
  ;[1 1 1] 播放开火特效_Multicast
  (`/Engine/EditorBlueprintResources/ActorMacros.Switch Has Authority`
    (:`Remote`
      (`ParticleSystemComponent.SetTemplate` (`self.射击特效`) (`self.枪口射击特效`)))))

(event `播放武器射击音效_Multicast`
  ;[1 1 1] 播放武器射击音效_Multicast
  (`/Engine/EditorBlueprintResources/ActorMacros.Switch Has Authority`
    (:`Remote`
      (`GameplayStatics.SpawnSoundAtLocation` (`self.射击音效`) (`self.K2_GetActorLocation`) (struct) 1.0 1.0 0.0 null null))))

(event `播放射击空枪音效_Multicast`
  ;[1 1 1] 播放射击空枪音效_Multicast
  (`/Engine/EditorBlueprintResources/ActorMacros.Switch Has Authority`
    (:`Remote`
      (`GameplayStatics.SpawnSoundAtLocation` "/Game/音效/射击音效_空枪.射击音效_空枪" (`self.K2_GetActorLocation`) (struct) 1.0 1.0 0.0 null null))))

(event `播放武器射击动画_Multicast`
  ;[1 1 1] 播放武器射击动画_Multicast
  (`SkeletalMeshComponent.PlayAnimation` (`self.SkeletalMesh`) (`self.武器射击动画`) false))

(fn `UserConstructionScript`)

(fn `射击`
  (params (`玩家摄像机数据` :type "/Game/结构数据/玩家摄像机数据_BP Structure"))
  (returns (`是否成功射击` :type Boolean))
  (bind _returnvalue (`KismetMathLibrary.GetForwardVector` `玩家摄像机数据_摄像机旋转体_5_D3766D15467AA6D8A10462B89C939FD0`))
  (bind _returnvalue_location (`KismetMathLibrary.BreakTransform` (`SceneComponent.GetSocketTransform` (`self.SkeletalMesh`) "Fire_FX_Slot" "RTS_World")))
  (bind _returnvalue_2 (`SceneComponent.GetSocketTransform` (`self.SkeletalMesh`) "子弹壳插槽" "RTS_World"))
  (`self.播放武器射击动画_Multicast`)
  (`SkeletalMeshComponent.PlayAnimation` (`self.SkeletalMesh`) (`self.武器射击动画`) false)
  (if (== (`self.弹匣子弹数量`) 0)
    (`self.播放射击空枪音效_Multicast`)
    (`GameplayStatics.SpawnSoundAtLocation` "/Game/音效/射击音效_空枪.射击音效_空枪" (`self.K2_GetActorLocation`) (struct) 1.0 1.0 0.0 null null)
    (return false)
    (else
      (`self.播放武器射击音效_Multicast`)
      (`GameplayStatics.SpawnSoundAtLocation` (`self.射击音效`) (`self.K2_GetActorLocation`) (struct) 1.0 1.0 0.0 null null)
      (`self.播放开火特效_Multicast`)
      (`ParticleSystemComponent.SetTemplate` (`self.射击特效`) (`self.枪口射击特效`))
      (`/Engine/EditorBlueprintResources/StandardMacros.DecrementInt` (`self.弹匣子弹数量`)
        (:`  `
          (bind (_outhit _returnvalue_3) (`KismetSystemLibrary.LineTraceSingle` (+ `玩家摄像机数据_摄像机位置_2_8BEC34B84B2C03606764B3A1E298D133` (* _returnvalue 100)) (+ `玩家摄像机数据_摄像机位置_2_8BEC34B84B2C03606764B3A1E298D133` (* _returnvalue 200000)) "TraceTypeQuery5"))
          (bind (_bblockinghit _binitialoverlap _time _distance _location _impactpoint _normal _impactnormal _physmat _hitactor _hitcomponent _hitbonename _bonename _hititem _elementindex _faceindex _tracestart _traceend) (`GameplayStatics.BreakHitResult` _outhit))
          (bind _returnvalue_4 (`|SpawnActorFromClass` "/Game/武器蓝图/子弹_BP.子弹_BP_C" (`KismetMathLibrary.MakeTransform` _returnvalue_location (`KismetMathLibrary.FindLookAtRotation` _returnvalue_location (select `bool` _returnvalue_3 :`false` _traceend :`true` _location))) "AlwaysSpawn" "MultiplyWithRoot" (`self.GetOwner`) (`self.GetInstigator`)))
          (set `/Game/武器蓝图/子弹_BP.攻击力` (`/Game/数据资产/武器_数据资产.攻击力` (`self.武器数据资产`)) _returnvalue_4)
          (`|SpawnActorFromClass` "/Game/武器蓝图/子弹壳_BP.子弹壳_BP_C" (`KismetMathLibrary.MakeTransform` (.location _returnvalue_2) (`KismetMathLibrary.MakeRotator` (.roll (.rotation _returnvalue_2)) (- (.pitch (.rotation _returnvalue_2)) (`KismetMathLibrary.RandomFloatInRange` -30.0 30.0)) (.yaw (.rotation _returnvalue_2))) (.scale _returnvalue_2)) "AlwaysSpawn" "MultiplyWithRoot" null null)
          (return true))))))

(fn `获取武器数据资产`
  (returns (`武器数据资产` :type "/Game/数据资产/武器_数据资产 Object Reference"))
  (return (`self.武器数据资产`)))