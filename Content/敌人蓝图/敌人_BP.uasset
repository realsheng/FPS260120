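; Enemy character that chases seen players and deals contact damage, with gameplay logic running on the server.
; PawnSensing triggers an AI move toward the seen pawn; capsule hits damage 玩家_BP, then a timer resets the attack cooldown.
; BeginPlay sets speed and health and links the 血条 health bar widget to itself on authority.
; Damage lowers health and destroys the actor at zero, while a RepNotify prints health on remotes.
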(event `死亡销毁`
  ;[1 1 1] 死亡销毁
  (`/Engine/EditorBlueprintResources/ActorMacros.Switch Has Authority`
    (:`Authority`
      (if (<= (`self.生命值`) 0)
        (`self.K2_DestroyActor`)))))

(event `生命值降低`
  (params (`伤害数值` :type Integer))
  (bind `_生命值` (`self.生命值`))
  ;[1 1 1] 生命值降低
  (`/Engine/EditorBlueprintResources/ActorMacros.Switch Has Authority`
    (:`Authority`
      (if (>= `_生命值` 0)
        (set `self.生命值` (- `_生命值` `伤害数值`))
        (else
          (set `self.生命值` 0)))
      (`self.死亡销毁`))))

(event `self.ReceiveBeginPlay`
  ;[1 1 1] 事件开始运行
  (set `CharacterMovementComponent.MaxWalkSpeed` 300.0 (`self.CharacterMovement`))
  (`/Engine/EditorBlueprintResources/ActorMacros.Switch Has Authority`
    (:`Authority`
      (bind _output_get (set `self.最大生命值` 200))
      (set `self.生命值` _output_get)
      (bind `_as血条` (cast `/Game/HUD/血条` (`WidgetComponent.GetWidget` (`self.Widget`))))
      (set `/Game/HUD/血条.所属角色` self `_as血条`)
      (set `self.攻击间隔` 2)
      (`self.攻击重置`))))

(event `self.PawnSensing.OnSeePawn`
  (params (Pawn :type "Pawn Object Reference"))
  ;[1 1 1] 看见pawn，移至pawn
  (`/Engine/EditorBlueprintResources/ActorMacros.Switch Has Authority`
    (:`Authority`
      (set `self.是否看见玩家` true)
      (`self.移动至玩家`))))

(event `移动至玩家`
  ;[1 1 1] 看见pawn，移至pawn
  (`/Engine/EditorBlueprintResources/ActorMacros.Switch Has Authority`
    (:`Authority`
      (if (`self.是否看见玩家`)
        (`|AIMoveTo` self (0.0 0.0 0.0) (stale `self.PawnSensing.OnSeePawn` Pawn))))))

(event `self.CapsuleComponent.OnComponentHit`
  (params (HitComponent :type "PrimitiveComponent Object Reference") (OtherActor :type "Actor Object Reference") (OtherComp :type "PrimitiveComponent Object Reference") (NormalImpulse :type "Vector Structure") (Hit :type "HitResult Structure (by ref)"))
  ;[1 1 1] 组件命中时
  (`/Engine/EditorBlueprintResources/ActorMacros.Switch Has Authority`
    (:`Authority`
      (`self.是否可以攻击`
        (:`then`
          (bind `_as玩家_bp` (cast `/Game/玩家蓝图/玩家_BP` OtherActor))
          (`/Game/玩家蓝图/玩家_BP.生命值降低` `_as玩家_bp` 10)
          (set `self.是否可以攻击` false)
          (`KismetSystemLibrary.K2_SetTimerDelegate` (delegate `攻击重置`) (`KismetMathLibrary.Conv_IntToDouble` (`self.攻击间隔`))))
        (:`else`)))))

(event `攻击重置`
  ;[1 1 1] 攻击重置
  (`/Engine/EditorBlueprintResources/ActorMacros.Switch Has Authority`
    (:`Authority`
      (set `self.是否可以攻击` true)
      (`KismetSystemLibrary.PrintString` "攻击重置"))))

(fn `OnRep_生命值`
  (`/Engine/EditorBlueprintResources/ActorMacros.Switch Has Authority`
    (:`Remote`
      (`KismetSystemLibrary.PrintString` (`KismetStringLibrary.Conv_IntToString` (`self.生命值`))))))

(fn `UserConstructionScript`)